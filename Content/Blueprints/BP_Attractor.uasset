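; BP_Attractor is an actor that alters the gravity scale of Characters that enter its box volume or hit its static mesh.
; Entering the box raises gravity scale sharply, and a mesh hit sets it to a somewhat lower but still heavy value.
; Leaving the box sets a fixed low gravity scale rather than restoring the Character's previous value.
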(event `self.Box.OnComponentBeginOverlap`
  (params (OverlappedComponent :type "PrimitiveComponent Object Reference") (OtherActor :type "Actor Object Reference") (OtherComp :type "PrimitiveComponent Object Reference") (OtherBodyIndex :type Integer) (bFromSweep :type Boolean) (SweepResult :type "HitResult Structure (by ref)"))
  (bind _ascharacter (cast `Character` OtherActor))
  (set `CharacterMovementComponent.GravityScale` 3.5 (`Character.CharacterMovement` _ascharacter)))

(event `self.Box.OnComponentEndOverlap`
  (params (OverlappedComponent :type "PrimitiveComponent Object Reference") (OtherActor :type "Actor Object Reference") (OtherComp :type "PrimitiveComponent Object Reference") (OtherBodyIndex :type Integer))
  (bind _ascharacter (cast `Character` OtherActor))
  (set `CharacterMovementComponent.GravityScale` 0.5 (`Character.CharacterMovement` _ascharacter)))

(event `self.StaticMeshComponent.OnComponentHit`
  (params (HitComponent :type "PrimitiveComponent Object Reference") (OtherActor :type "Actor Object Reference") (OtherComp :type "PrimitiveComponent Object Reference") (NormalImpulse :type "Vector Structure") (Hit :type "HitResult Structure (by ref)"))
  (bind _ascharacter (cast `Character` OtherActor))
  (set `CharacterMovementComponent.GravityScale` 2.5 (`Character.CharacterMovement` _ascharacter)))

(fn `UserConstructionScript`)